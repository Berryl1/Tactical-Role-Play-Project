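; Parent Blueprint for playable characters, providing tile-style movement on a bounded grid.
; Four custom events step the SkeletalMesh one fixed-size cell up, down, left or right by teleporting it without sweep.
; XPosition and YPostion track the current cell and gate each move at the grid edges.
; Only the mesh component is moved, not the actor; BeginPlay, Tick, overlap and construction script are empty.
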(event `Move UP`
  (bind _skeletalmesh (`self.SkeletalMesh`))
  ;[1 1 1] Move
  (if (< (`self.Y Postion`) 3)
    (`SceneComponent.K2_SetWorldLocation` _skeletalmesh (+ (`SceneComponent.K2_GetComponentLocation` _skeletalmesh) (100.0 0.0 0.0)) false true)
    (set `self.Y Postion` (+ (`self.Y Postion`) 1))))

(event `Move Down`
  (bind _skeletalmesh (`self.SkeletalMesh`))
  ;[1 1 1] Move
  (if (> (`self.Y Postion`) 1)
    (`SceneComponent.K2_SetWorldLocation` _skeletalmesh (+ (`SceneComponent.K2_GetComponentLocation` _skeletalmesh) (-100.0 0.0 0.0)) false true)
    (set `self.Y Postion` (- (`self.Y Postion`) 1))))

(event `Move Left`
  (bind _skeletalmesh (`self.SkeletalMesh`))
  ;[1 1 1] Move
  (if (> (`self.X Position`) -3)
    (`SceneComponent.K2_SetWorldLocation` _skeletalmesh (+ (`SceneComponent.K2_GetComponentLocation` _skeletalmesh) (0.0 -100.0 0.0)) false true)
    (set `self.X Position` (- (`self.X Position`) 1))))

(event `Move Right`
  (bind _skeletalmesh (`self.SkeletalMesh`))
  ;[1 1 1] Move
  (if (< (`self.X Position`) 3)
    (`SceneComponent.K2_SetWorldLocation` _skeletalmesh (+ (`SceneComponent.K2_GetComponentLocation` _skeletalmesh) (0.0 100.0 0.0)) false true)
    (set `self.X Position` (+ (`self.X Position`) 1))))

(fn `UserConstructionScript`)