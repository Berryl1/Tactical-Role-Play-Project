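; PlayController_BP is a player controller, apparently for testing, that shows the mouse cursor and puts Test_WDG on screen at BeginPlay.
; Debug key T finds a Pareents_BP actor and teleports its skeletal mesh along world Y by a fixed step.
; Debug key Q creates and displays a new Select_Widget on each press, with no guard against duplicates.
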(event EventBeginPlay
  (Variables|Default|SetbShowMouseCursor true)
  (bind _returnvalue (UserInterface|CreateWidget "/Game/_UI/Test_WDG.Test_WDG_C"))
  (UserInterface|Viewport|AddtoViewport _returnvalue 0))

(event EventTick
  (params (DeltaSeconds :type Float%20%28single-precision%29)))

(event Input|KeyboardEvents|DebugKeyQ
  (params (Key :type Key%20Structure :default "None") (ActionValue :type Input%20Action%20Value%20Structure))
  ;[1 1 1] 한번만 눌러
  (:Pressed
    (bind _returnvalue (UserInterface|CreateWidget "/Game/_UI/Select_Widget.Select_Widget_C"))
    (UserInterface|Viewport|AddtoViewport _returnvalue 0)))

(event Input|KeyboardEvents|DebugKeyT
  (params (Key :type Key%20Structure :default "None") (ActionValue :type Input%20Action%20Value%20Structure))
  (:Pressed
    (bind _returnvalue (Actor|GetActorOfClass "/Game/_PlayChar/Pareents_BP.Pareents_BP_C"))
    (Transformation|SetWorldLocation (Variables|/Game/_PlayChar/Pareents_BP.Pareents_BP_C|GetSkeletalMesh _returnvalue) (+ (Transformation|GetWorldLocation (Variables|/Game/_PlayChar/Pareents_BP.Pareents_BP_C|GetSkeletalMesh _returnvalue)) "0.000000,100.000000,0.000000") false true)))

(fn ConstructionScript)